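; Base human character Blueprint for saber combat, turning state changes and combat events into animation and input control.
; State changes lock or restore movement, start or stop the sword-blocking montage, and disable input on death.
; Combat toggling routes through server and multicast events, holding ChangingCombat while the saber opens or closes with draw or sheath montages.
; It also forwards jump press/release, plays saber-throw and death animations, and exposes starting stats and saber flight distance.
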(event `self.OnChangeState`
  (params (NewState :type "EHumanState Enum" :default "EHS_Stunned"))
  (bind _returnvalue (`self.GetController`))
  (bind _returnvalue_2 (`self.GetController`))
  (switch `EHumanState` NewState
    (:`EHS_Stunned`
      (`/Engine/EditorBlueprintResources/StandardMacros.IsValid` _returnvalue_2 :!label _label
        (:`Is Valid`
          (`Controller.SetIgnoreMoveInput` _returnvalue_2 true))))
    (:`EHS_Impacted`
      (goto _label))
    (:`EHS_Free`
      (bind _asanim_bp_eve (cast `/Game/Characters/Eve/Animations/AnimBP_Eve` (`SkeletalMeshComponent.GetAnimInstance` (`self.Mesh`)))
        (:`then`
          (bind _returnvalue_3 (`AnimInstance.GetCurrentActiveMontage` _asanim_bp_eve))
          (if (== _returnvalue_3 "/Game/Characters/Eve/Animations/Montages/SwordBlocking_Montage.SwordBlocking_Montage")
            (`AnimInstance.Montage_Stop` _asanim_bp_eve 0.0 _returnvalue_3)))
        (:`CastFailed`
          _))
      (if (`KismetSystemLibrary.IsValid` _returnvalue) :!label _label_2
        (`Controller.SetIgnoreMoveInput` _returnvalue false)))
    (:`EHS_Attacking`
      (goto _label_2))
    (:`EHS_Acrobatic`
      (goto _label_2))
    (:`EHS_ChangingCombat`
      (goto _label_2))
    (:`EHS_Defending`
      (bind _asanim_bp_eve_2 (cast `/Game/Characters/Eve/Animations/AnimBP_Eve` (`SkeletalMeshComponent.GetAnimInstance` (`self.Mesh`))))
      (`AnimInstance.Montage_Play` _asanim_bp_eve_2 "/Game/Characters/Eve/Animations/Montages/SwordBlocking_Montage.SwordBlocking_Montage" 1.0 "Duration" 0.0 true))
    (:`EHS_Dead`
      (`self.DisableInput` (`GameplayStatics.GetPlayerController` 0)))))

(event `Key|SpaceBar`
  (params (Key :type "Key Structure"))
  ;[1 1 1] Jump duration handling
  (:`Pressed`
    (`self.SpacePressed`))
  (:`Released`
    (`self.SpaceReleased`)))

(event `Multicast_ToggleCombat`
  (params (NewParam :type Boolean))
  (bind _returnvalue (`self.GetSaber`))
  ;[1 1 1] Toggling saber show/hide
  (if (`|EnumEquality` (`self.GetState`) "EHS_Free")
    (`self.SetState` "EHS_ChangingCombat")
    (bind _asanim_bp_eve (cast `/Game/Characters/Eve/Animations/AnimBP_Eve` (`SkeletalMeshComponent.GetAnimInstance` (`self.Mesh`))))
    (if NewParam
      (`Saber.SetSaberState` _returnvalue "ESS_Opening")
      (bind _returnvalue_2 (`AnimInstance.Montage_Play` _asanim_bp_eve "/Game/Characters/Eve/Animations/Montages/Draw_Sword_Montage.Draw_Sword_Montage" 1.0 "MontageLength" 0.0 true))
      (`KismetSystemLibrary.Delay` _returnvalue_2)
      (else
        (`Saber.SetSaberState` _returnvalue "ESS_Closing")
        (bind _returnvalue_3 (`AnimInstance.Montage_Play` _asanim_bp_eve "/Game/Characters/Eve/Animations/Montages/Sheath_Sword_Montage.Sheath_Sword_Montage" 1.0 "MontageLength" 0.0 true))
        (`KismetSystemLibrary.Delay` _returnvalue_3)))
    (`self.SetState` "EHS_Free")))

(event `self.OnToggleCombat`
  (params (NewCombatState :type Boolean))
  ;[1 1 1] Toggling saber show/hide
  ;;[1 1 1] Network saber show\hide
  (`/Engine/EditorBlueprintResources/ActorMacros.Switch Has Authority`
    (:`Authority`
      (`self.Multicast_ToggleCombat` NewCombatState))
    (:`Remote`
      (`self.Server_ToggleCombat` NewCombatState))))

(event `Server_ToggleCombat`
  (params (NewParam :type Boolean))
  ;[1 1 1] Toggling saber show/hide
  ;;[1 1 1] Network saber show\hide
  (`self.Multicast_ToggleCombat` NewParam))

(event `self.OnThrowSaber`
  ;[1 1 1] On saber throw hand animation
  (bind _asanim_bp_eve (cast `/Game/Characters/Eve/Animations/AnimBP_Eve` (`SkeletalMeshComponent.GetAnimInstance` (`self.Mesh`))))
  (`AnimInstance.Montage_Play` _asanim_bp_eve "/Game/Characters/Eve/Animations/SaberThrow_Montage.SaberThrow_Montage" 1.0 "Duration" 0.0 true))

(event `Die`
  (params (DiedHuman :type "Human Object Reference"))
  ;[1 1 1] Stops all animations and playes death animation
  (`AnimInstance.Montage_Stop` (`SkeletalMeshComponent.GetAnimInstance` (`self.Mesh`)) 0.0 null)
  (`/Engine/EditorBlueprintResources/StandardMacros.IsValid` (`self.DeathAnimation`)
    (:`Is Valid`
      (`SkeletalMeshComponent.PlayAnimation` (`self.Mesh`) "/Game/Characters/Eve/Animations/Death.Death" false))
    (:`Is Not Valid`
      (`KismetSystemLibrary.PrintString` (`KismetStringLibrary.Concat_StrStr` (`KismetSystemLibrary.GetDisplayName` self) " has no death animaition assigned") true true (struct :`R` 1.0 :`B` 0.570817 :`A` 1.0) 10.0))))

(fn `GetMaxSaberFlyDistance`
  (returns (MaxDistance :type "Float (double-precision)"))
  (return (`self.MaxSaberFlyDistance`)))

(fn `GetStartingStats`
  (returns (CurStats :type "HumanStats Structure"))
  (return (`self.StartingStats`)))

(fn `UserConstructionScript`)
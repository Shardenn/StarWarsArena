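; BP_Saber is a lightsaber Blueprint that adds sound and light feedback to saber states and blade hits.
; State changes drive turn-on, idle and turn-off audio and toggle the point light; initialization starts closing the saber.
; Blade overlap results from C++ replicate hit audio via multicast, routed through a server RPC for remote callers, though only Damage and Cancel selections are handled.
; The Blueprint's own overlap handler does nothing.
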(event `Multicast_PlayHitSound`
  (params (Selection :type "EBladeOverlapResult Enum" :default "EBOR_PlayerMesh"))
  ;[1 1 1] Blade overlap replicating sound play
  (switch `EBladeOverlapResult` Selection
    (:`EBOR_DamageCancel`
      (`AudioComponent.Play` (`self.Lightsaber_randomHit`) 0.0))))

(event `Server_PlayHitSound`
  (params (Selection :type "EBladeOverlapResult Enum" :default "EBOR_PlayerMesh"))
  ;[1 1 1] Blade overlap replicating sound play
  (`self.Multicast_PlayHitSound` Selection))

(event `self.OnBladeOverlapCPP`
  (params (Result :type "EBladeOverlapResult Enum" :default "EBOR_PlayerMesh"))
  ;[1 1 1] Blade overlap replicating sound play
  (`/Engine/EditorBlueprintResources/ActorMacros.Switch Has Authority`
    (:`Authority`
      (`self.Multicast_PlayHitSound` Result))
    (:`Remote`
      (`self.Server_PlayHitSound` Result))))

(event `self.OnSaberChangeState`
  (params (NewState :type "ESaberState Enum" :default "ESS_Opened"))
  (bind _lightsaber_idle_cue (`self.Lightsaber_idle_Cue`))
  (switch `ESaberState` NewState
    (:`ESS_Opened`
      (if (not (`AudioComponent.IsPlaying` _lightsaber_idle_cue))
        (`AudioComponent.Play` _lightsaber_idle_cue 0.0)))
    (:`ESS_Closed`
      (`SceneComponent.ToggleVisibility` (`self.PointLight`) false))
    (:`ESS_Opening`
      (`SceneComponent.ToggleVisibility` (`self.PointLight`) false)
      (`AudioComponent.Play` (`self.Lightsaber_turn_ON_01`) 0.0))
    (:`ESS_Closing`
      (`KismetSystemLibrary.Delay` 0.25)
      (`AudioComponent.Stop` (`self.Lightsaber_idle_Cue`))
      (`AudioComponent.Play` (`self.Lightsaber_turnOFF`) 0.0))
    (:`ESS_Flying`)
    (:`ESS_Returning`)))

(event `self.Blade.OnComponentBeginOverlap`
  (params (OverlappedComponent :type "PrimitiveComponent Object Reference") (OtherActor :type "Actor Object Reference") (OtherComp :type "PrimitiveComponent Object Reference") (OtherBodyIndex :type Integer) (bFromSweep :type Boolean) (SweepResult :type "HitResult Structure (by ref)"))
  (if (`|EnumEquality` (`self.GetSaberState`) "ESS_Opened")
    _))

(event `InitializeSaber`
  (`self.CloseSaber`))

(event `CloseSaber`
  (`self.SetSaberState` "ESS_Closing"))

(fn `PlaySwingSound`
  (`AudioComponent.Play` (`self.Lightsaber_swing`) 0.0))

(fn `UserConstructionScript`)
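; BP_Human is the player character Blueprint for a saber-wielding human, handling combat states, animation and saber networking.
; State changes lock movement input when stunned or impacted and start or stop the blocking montage.
; On non-authority BeginPlay it requests a server saber spawn, then multicasts attachment to the belt.
; Combat toggles route to the server, opening or closing the saber and holding ChangingCombat for the draw or sheath montage's length.
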(event `self.OnChangeState`
  (params (NewState :type "EHumanState Enum" :default "EHS_Stunned"))
  (bind _returnvalue (`self.GetController`))
  (bind _returnvalue_2 (`self.GetController`))
  (switch `EHumanState` NewState
    (:`EHS_Stunned`
      (`/Engine/EditorBlueprintResources/StandardMacros.IsValid` _returnvalue_2 :!label _label
        (:`Is Valid`
          (`Controller.SetIgnoreMoveInput` _returnvalue_2 true))))
    (:`EHS_Impacted`
      (goto _label))
    (:`EHS_Free`
      (bind _asanim_bp_eve (cast `/Game/Characters/Eve/Animations/AnimBP_Eve` (`SkeletalMeshComponent.GetAnimInstance` (`self.Mesh`)))
        (:`then`
          (bind _returnvalue_3 (`AnimInstance.GetCurrentActiveMontage` _asanim_bp_eve))
          (if (== _returnvalue_3 "/Game/Characters/Eve/Animations/Montages/SwordBlocking_Montage.SwordBlocking_Montage")
            (`AnimInstance.Montage_Stop` _asanim_bp_eve 0.0 _returnvalue_3)))
        (:`CastFailed`
          _))
      (if (`KismetSystemLibrary.IsValid` _returnvalue) :!label _label_2
        (`Controller.SetIgnoreMoveInput` _returnvalue false)))
    (:`EHS_Attacking`
      (goto _label_2))
    (:`EHS_Acrobatic`
      (goto _label_2))
    (:`EHS_ChangingCombat`
      (goto _label_2))
    (:`EHS_Defending`
      (bind _asanim_bp_eve_2 (cast `/Game/Characters/Eve/Animations/AnimBP_Eve` (`SkeletalMeshComponent.GetAnimInstance` (`self.Mesh`))))
      (`AnimInstance.Montage_Play` _asanim_bp_eve_2 "/Game/Characters/Eve/Animations/Montages/SwordBlocking_Montage.SwordBlocking_Montage" 1.0 "Duration" 0.0))))

(event `Key|SpaceBar`
  (params (Key :type "Key Structure"))
  ;[1 1 1] Jump duration handling
  (:`Pressed`
    (`self.SpacePressed`))
  (:`Released`
    (`self.SpaceReleased`)))

(event `Multicast_SetSaber`
  (params (SpawnedSaber :type "Saber Object Reference"))
  ;[1 1 1] Attach saber from class to player
  (`self.SetSaber` SpawnedSaber)
  (`Saber.SetHuman` SpawnedSaber self)
  (`self.PutSaberInBelt`))

(event `self.ReceiveBeginPlay`
  ;[1 1 1] Attach saber from class to player
  (`/Engine/EditorBlueprintResources/ActorMacros.Switch Has Authority`
    (:`Remote`
      (`self.Server_SaberSpawn` (`self.SaberClassToSpawn`)))))

(event `Server_SaberSpawn`
  (params (ClassToSpawn :type "Saber Class Reference"))
  ;[1 1 1] Attach saber from class to player
  (bind _returnvalue (`|SpawnActorFromClass` ClassToSpawn (`KismetMathLibrary.MakeTransform` (+ (`self.K2_GetActorLocation`) (0.0 0.0 150.0))) "AlwaysSpawn" "OverrideRootScale" self null))
  (`self.Server_AddOwner` _returnvalue)
  (`self.Multicast_SetSaber` _returnvalue))

(event `Server_AddOwner`
  (params (ChildWithNewOwner :type "Actor Object Reference"))
  ;[1 1 1] Attach saber from class to player
  (`self.SetOwner` ChildWithNewOwner (`self.GetController`)))

(event `Server_ToggleCombat`
  (params (NewParam :type Boolean))
  (bind _returnvalue (`self.GetSaber`))
  ;[1 1 1] Toggling saber show/hide
  (if (`|EnumEquality` (`self.GetState`) "EHS_Free")
    (`self.SetState` "EHS_ChangingCombat")
    (bind _asanim_bp_eve (cast `/Game/Characters/Eve/Animations/AnimBP_Eve` (`SkeletalMeshComponent.GetAnimInstance` (`self.Mesh`))))
    (if NewParam
      (`Saber.SetSaberState` _returnvalue "ESS_Opening")
      (bind _returnvalue_2 (`AnimInstance.Montage_Play` _asanim_bp_eve "/Game/Characters/Eve/Animations/Montages/Draw_Sword_Montage.Draw_Sword_Montage" 1.0 "MontageLength" 0.0))
      (`KismetSystemLibrary.Delay` _returnvalue_2)
      (else
        (`Saber.SetSaberState` _returnvalue "ESS_Closing")
        (bind _returnvalue_3 (`AnimInstance.Montage_Play` _asanim_bp_eve "/Game/Characters/Eve/Animations/Montages/Sheath_Sword_Montage.Sheath_Sword_Montage" 1.0 "MontageLength" 0.0))
        (`KismetSystemLibrary.Delay` _returnvalue_3)))
    (`self.SetState` "EHS_Free")))

(event `self.OnToggleCombat`
  (params (NewCombatState :type Boolean))
  ;[1 1 1] Toggling saber show/hide
  ;;[1 1 1] Network saber show\hide
  (`/Engine/EditorBlueprintResources/ActorMacros.Switch Has Authority`
    (:`Authority`
      (`self.Server_ToggleCombat` NewCombatState))
    (:`Remote`
      (`self.Client_ToggleCombat` NewCombatState))))

(event `Client_ToggleCombat`
  (params (NewParam :type Boolean))
  ;[1 1 1] Toggling saber show/hide
  ;;[1 1 1] Network saber show\hide
  (`self.Server_ToggleCombat` NewParam))

(event `self.OnThrowSaber`
  ;[1 1 1] On saber throw hand animation
  (bind _asanim_bp_eve (cast `/Game/Characters/Eve/Animations/AnimBP_Eve` (`SkeletalMeshComponent.GetAnimInstance` (`self.Mesh`))))
  (`AnimInstance.Montage_Play` _asanim_bp_eve "/Game/Characters/Eve/Animations/SaberThrow_Montage.SaberThrow_Montage" 1.0 "Duration" 0.0))

(fn `GetMaxSaberFlyDistance`
  (returns (MaxDistance :type "Float (double-precision)"))
  (return (`self.MaxSaberFlyDistance`)))

(fn `GetStartingStats`
  (returns (CurStats :type "HumanStats Structure"))
  (return (`self.StartingStats`)))

(fn `UserConstructionScript`)